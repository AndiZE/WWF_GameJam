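; Base building actor for a tile-based game, with Green, Dirty and Abandoned states that drive pollution.
; ActivateToGrid line-traces down across its tile footprint to register itself on the GameInstance map and starts a decay timer.
; Cash-gated upgrades and timer-capable downgrades step the state, updating greenery visibility, dirt material parameter, pollution component and UI.
; Clicking highlights the mesh and shows its tile in the player's UI.
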(event OnClicked(StaticMeshComponent)
  (params (TouchedComponent :type Primitive%20Component%20Object%20Reference) (ButtonPressed :type Key%20Structure :default "None"))
  (Rendering|Material|SetScalarParameterValueonMaterials (Variables|Debug|GetStaticMeshComponent) "Selection" 1.0)
  (CallFunction|UpdateUI))

(event EventBeginPlay
  (bind _asbp_debugplayer (Utilities|Casting|CastToBP_Debugplayer (Game|Player|GetPlayerPawn 0)))
  (Variables|Default|SetPlayer _asbp_debugplayer))

(fn ConstructionScript)

(fn ActivatetoGrid
  (bind _tilesize (Variables|Default|GetTileSize))
  (bind _tilesize_2 (Variables|Default|GetTileSize))
  (bind _asbp_game_instance (Utilities|Casting|CastToBP_GameInstance (Game|GetGameInstance)))
  (LocalVariables|SetGameInstance _asbp_game_instance)
  (if (== (Variables|Default|GetTileSizeX) 1)
    (LocalVariables|SetOffset (+ (LocalVariables|GetOffset) (Math|Vector|MakeVector (* (Variables|Default|GetTileSize) 0.5) 0.0 0.0))))
  (if (== (Variables|Default|GetTileSizeY) 1)
    (LocalVariables|SetOffset (+ (LocalVariables|GetOffset) (Math|Vector|MakeVector 0.0 (* (Variables|Default|GetTileSize) 0.5) 0.0))))
  (for _index (range 0 (- (Variables|Default|GetTileSizeY) 1)) ; y
    (for _index_2 (range 0 (- (Variables|Default|GetTileSizeX) 1)) ; x
      (bind _outhit (Collision|LineTraceByChannel (+ (Transformation|GetActorLocation) (Math|Vector|MakeVector (- (* _index_2 _tilesize) (* _tilesize 0.5)) (- (* _index _tilesize_2) (* _tilesize_2 0.5)) 0.0) (LocalVariables|GetOffset)) (+ (+ (Transformation|GetActorLocation) (Math|Vector|MakeVector (- (* _index_2 _tilesize) (* _tilesize 0.5)) (- (* _index _tilesize_2) (* _tilesize_2 0.5)) 0.0) (LocalVariables|GetOffset)) (* (Transformation|GetActorUpVector) -4e+02)) "TraceTypeQuery1" false 0 "None"))
      (Default|SetBuilding (Default|GetTilefromWorldPosition (Variables|/Game/GameMode/BP_GameInstance.BP_GameInstance_C|GetMap (LocalVariables|GetGameInstance)) (.Location (Collision|BreakHitResult _outhit))) self)
      (bind _returnvalue (Utilities|Time|SetTimerbyEvent (EventDispatchers|CreateEvent :!event DowngradeBuilding) (Variables|Default|GetDecayTime)))
      (Variables|Default|SetDecayTimer _returnvalue)
      (Rendering|SetVisibility (Variables|Default|GetGruen) false false))))

(fn UpgradeBuilding
  (if (Utilities|Enum|NotEqual(Enum) (Variables|Default|GetState) "NewEnumerator0")
    (bind _success (Default|CanSpendCash (Variables|Default|GetPlayer) (Variables|/Game/Blueprint/Tiles/BPC_Cash.BPC_Cash_C|GetUpgradeCost (Variables|Default|GetBPC_Cash))))
    (if _success
      (switch Utilities|FlowControl|Switch|SwitchonEBuildingState (Variables|Default|GetState)
        (:NewEnumerator1
          (Variables|Default|SetState "NewEnumerator0")
          (Rendering|SetVisibility (Variables|Default|GetGruen) true false)
          (Rendering|Material|SetScalarParameterValueonMaterials (Variables|Debug|GetStaticMeshComponent) "DirtOverlay" 0.0)
          (Utilities|Time|ClearandInvalidateTimerbyHandle (Variables|Default|GetDecayTimer)))
        (:NewEnumerator2
          (Variables|Default|SetState "NewEnumerator1")
          (Rendering|Material|SetScalarParameterValueonMaterials (Variables|Debug|GetStaticMeshComponent) "DirtOverlay" 0.5)
          (bind _returnvalue (Utilities|Time|SetTimerbyEvent (EventDispatchers|CreateEvent :!event DowngradeBuilding) (Variables|Default|GetDecayTime)))
          (Variables|Default|SetDecayTimer _returnvalue)))
      (Default|SwitchPollution (Variables|Default|GetBPC_Pollution) (Variables|Default|GetState))
      (CallFunction|UpdateUI))))

(fn UpdateUI
  (bind _asbp_game_instance (Utilities|Casting|CastToBP_GameInstance (Game|GetGameInstance)))
  (Default|SelectedTile (Variables|Default|GetPlayer) (Default|GetTilefromWorldPosition (Variables|/Game/GameMode/BP_GameInstance.BP_GameInstance_C|GetMap _asbp_game_instance) (Transformation|GetActorLocation))))

(fn DowngradeBuilding
  (if (Utilities|Enum|NotEqual(Enum) (Variables|Default|GetState) "NewEnumerator2")
    (switch Utilities|FlowControl|Switch|SwitchonEBuildingState (Variables|Default|GetState)
      (:NewEnumerator0
        (Variables|Default|SetState "NewEnumerator1")
        (Rendering|SetVisibility (Variables|Default|GetGruen) false false)
        (Rendering|Material|SetScalarParameterValueonMaterials (Variables|Debug|GetStaticMeshComponent) "DirtOverlay" 0.5))
      (:NewEnumerator1
        (Variables|Default|SetState "NewEnumerator2")
        (Utilities|Time|ClearandInvalidateTimerbyHandle (Variables|Default|GetDecayTimer))
        (Rendering|Material|SetScalarParameterValueonMaterials (Variables|Debug|GetStaticMeshComponent) "DirtOverlay" 0.5)))
    (Default|SwitchPollution (Variables|Default|GetBPC_Pollution) (Variables|Default|GetState))
    (CallFunction|UpdateUI)))

(fn DecayBuilding
  (CallFunction|DowngradeBuilding))