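; Map manager actor for a tile-based building game with taxes and pollution-based win and lose conditions.
; On BeginPlay it builds a grid of linked O_Tile objects, registers itself and camera bounds with the game instance, activates placed buildings, and starts a looping tax timer.
; CollectTax pays the player income from unique, non-upgrading buildings.
; Tick sums tile pollution to update the HUD and road dirtiness material parameter and show end screens.
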(event EventBeginPlay
  (bind _returnvalue (Transformation|GetActorLocation))
  (bind _gridsize (Variables|Map|GetGridsize))
  (Utilities|FlowControl|Sequence
    (:then_0
      ;[1 1 1] Map Generation
      (bind _asbp_game_instance (Utilities|Casting|CastToBP_GameInstance (Game|GetGameInstance)))
      (Variables|/Game/GameMode/BP_GameInstance.BP_GameInstance_C|SetMap _asbp_game_instance self)
      (CallFunction|CreateGrid)
      (Variables|/Game/GameMode/BP_GameInstance.BP_GameInstance_C|SetCamMinPos _asbp_game_instance _returnvalue)
      (Variables|/Game/GameMode/BP_GameInstance.BP_GameInstance_C|SetCamMaxPos _asbp_game_instance (+ _returnvalue (Math|Vector|MakeVector (* (Variables|Map|GetSizeX) _gridsize) (* (Variables|Map|GetSizeY) _gridsize) 0.0))))
    (:then_1
      ;[1 1 1] Taxes
      (bind _returnvalue_2 (Utilities|Time|SetTimerbyEvent (EventDispatchers|CreateEvent :!event CollectTax) (Variables|Default|GetTaxInterval) true))
      (Variables|Default|SetTaxTimer _returnvalue_2))
    (:then_2
      (Audio|PlaySound2D "/Game/Audio/Creepy_Ambience_LOOP.Creepy_Ambience_LOOP" 1.0 1.0 0.0 0 0))
    (:then_3
      (CallFunction|RegisterBuildings)
      (bind _returnvalue_3 (UserInterface|CreateWidget "/Game/UI/WBP_Tutorial.WBP_Tutorial_C"))
      (UserInterface|Viewport|AddtoViewport _returnvalue_3 3))))

(event EventTick
  (params (DeltaSeconds :type Float%20%28single-precision%29))
  (bind _asbp_debugplayer (Utilities|Casting|CastToBP_Debugplayer (Game|Player|GetPlayerPawn 0)))
  (Default|UpdateProgressBar (Variables|/Game/Player/BP_Debugplayer.BP_Debugplayer_C|GetInfoHud _asbp_debugplayer) (Variables|Default|GetTaxInterval) (Class|KismetSystemLibrary|GetTimerElapsedTimeHandle (Variables|Default|GetTaxTimer)))
  (bind _totalpollution (CallFunction|GetTotalPollution))
  (Default|UpdatePollution (Variables|/Game/Player/BP_Debugplayer.BP_Debugplayer_C|GetInfoHud _asbp_debugplayer) _totalpollution)
  (Rendering|Material|SetScalarParameterValue "/Game/Roads/Roadparameters.Roadparameters" "Dirtyness" (/ (Math|Conversions|ToFloat(Integer) _totalpollution) (Math|Conversions|ToFloat(Integer) (- (Variables|Default|GetLosePollutionThreshold) (Variables|Default|GetWinPollutionThreshold)))) :!class /Script/Engine.KismetMaterialLibrary)
  (if (<= _totalpollution (Variables|Default|GetWinPollutionThreshold)) ; Pollution WIn
    (Utilities|FlowControl|DoOnce false
      (:Completed
        (bind _returnvalue (UserInterface|CreateWidget "/Game/UI/WBP_Win.WBP_Win_C"))
        (UserInterface|Viewport|AddtoViewport _returnvalue 0)))
    (elif (>= _totalpollution (Variables|Default|GetLosePollutionThreshold)) ; Pollution Lose
      (Utilities|FlowControl|DoOnce false
        (:Completed
          (bind _returnvalue_2 (UserInterface|CreateWidget "/Game/UI/WBP_LosePollution.WBP_LosePollution_C"))
          (UserInterface|Viewport|AddtoViewport _returnvalue_2 0))))))

(fn ConstructionScript)

(fn CreateGrid
  (bind _gridsize (Variables|Map|GetGridsize))
  (bind _returnvalue (* _gridsize 0.5))
  (Variables|Map|SetStartPosition "0, 0, 0")
  (CallFunction|ClearGrid)
  (for _index (range 0 (- (Variables|Map|GetSizeY) 1)) ; Y
    (for _index_2 (range 0 (- (Variables|Map|GetSizeX) 1)) ; X
      (bind _returnvalue_2 (Game|ConstructObjectfromClass "/Game/Blueprint/Tiles/O_Tile.O_Tile_C" self _index_2 _index (+ (Variables|Map|GetStartPosition) (Math|Vector|MakeVector (+ (* _index_2 (Variables|Map|GetGridsize)) _returnvalue) (+ (* _index (Variables|Map|GetGridsize)) _returnvalue) 0.0))))
      (Utilities|FlowControl|Sequence
        (:then_0
          (if (> _index_2 0)
            (Default|SetNeighbour _returnvalue_2 (CallFunction|GetTilefromGridPosition (- _index_2 1) _index) "NewEnumerator2")))
        (:then_1
          (if (> _index 0)
            (Default|SetNeighbour _returnvalue_2 (CallFunction|GetTilefromGridPosition _index_2 (- _index 1)) "NewEnumerator3")))
        (:then_2
          (Utilities|Array|Add (Variables|Map|GetGridMap) _returnvalue_2))))))

(fn ClearGrid
  (for _array_element (Variables|Map|GetGridMap)
    (Utilities|Array|Clear (Variables|/Game/Blueprint/Tiles/O_Tile.O_Tile_C|GetNeighbours _array_element)))
  (Utilities|Array|Clear (Variables|Map|GetGridMap)))

(fn GetTilefromGridPosition
  (params (XPos :type Integer) (YPos :type Integer))
  (return (Utilities|Array|Get(acopy) (Variables|Map|GetGridMap) (+ (* YPos (Variables|Map|GetSizeX)) XPos))))

(fn GetTilePositionfromWorldPosition
  (params (WorldPosition :type Vector))
  (bind _returnvalue (Transformation|GetActorLocation))
  (bind _returnvalue_2 (- WorldPosition _returnvalue))
  (return (Math|Integer|Clamp(Integer) (Math|Float|Truncate (/ (.x _returnvalue_2) (Variables|Default|GetGridSize))) 0 (- (Variables|Map|GetSizeX) 1)) (Math|Integer|Clamp(Integer) (Math|Float|Truncate (/ (.y _returnvalue_2) (Variables|Default|GetGridSize))) 0 (- (Variables|Map|GetSizeY) 1))))

(fn GetTilefromWorldPosition
  (params (WorldPosition :type Vector))
  (bind (_xpos _ypos) (CallFunction|GetTilePositionfromWorldPosition WorldPosition))
  (return (CallFunction|GetTilefromGridPosition _xpos _ypos)))

(fn GetTotalPollution
  (for _array_element (Variables|Map|GetGridMap)
    (LocalVariables|SetPollution (+ (LocalVariables|GetPollution) (Default|GetPollution _array_element))))
  (return (LocalVariables|GetPollution)))

(fn CollectTax
  (for _array_element (Variables|Map|GetGridMap)
    (Utilities|IsValid (Default|GetBuilding _array_element)
      (:Is%20Valid
        (Utilities|Array|AddUnique (LocalVariables|GetBuildings) (Default|GetBuilding _array_element)))))
  (for _array_element_2 (LocalVariables|GetBuildings)
    (if (not (Default|IsUpgrading (Variables|/Game/Buildings/BP_BaseBuilding.BP_BaseBuilding_C|GetBPC_Cash _array_element_2)))
      (LocalVariables|SetTaxesCollected (+ (LocalVariables|GetTaxesCollected) (Default|GetIncome (Variables|/Game/Buildings/BP_BaseBuilding.BP_BaseBuilding_C|GetBPC_Cash _array_element_2) (Variables|/Game/Buildings/BP_BaseBuilding.BP_BaseBuilding_C|GetState _array_element_2))))))
  (bind _asbp_debugplayer (Utilities|Casting|CastToBP_Debugplayer (Game|Player|GetPlayerPawn 0)))
  (Default|AddCash _asbp_debugplayer (LocalVariables|GetTaxesCollected)))

(fn RegisterBuildings
  (bind _outactors (Actor|GetAllActorsOfClass "/Game/Buildings/BP_BaseBuilding.BP_BaseBuilding_C"))
  (for _array_element _outactors
    (Default|ActivatetoGrid _array_element)))

(fn FindTileswithBuilding
  (params (Building :type BP%20Base%20Building%20Object%20Reference))
  (for _array_element (Variables|Map|GetGridMap)
    (if (== (Default|GetBuilding _array_element) Building)
      (Utilities|Array|Add (LocalVariables|GetTile) _array_element)))
  (return (LocalVariables|GetTile)))