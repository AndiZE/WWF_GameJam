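; Grid helper library for tiles, with one function that gathers the tiles within a given number of neighbour steps of a start tile.
; GetTilesInRange expands outward once per range step, adding valid neighbours uniquely to a saved list.
; Each pass re-expands the whole saved list rather than only the newest ring, and the start tile enters the result only as another tile's neighbour.
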(fn GetTilesinRange
  (params (StartTile :type O%20Tile%20Object%20Reference) (Range :type Integer))
  (bind _output_get (LocalVariables|SetCounter Range))
  (Utilities|Array|Add (LocalVariables|Getopenlist) StartTile)
  (while (> _output_get 0)
    (Math|Integer|DecrementInt (LocalVariables|GetCounter)
      (:%20%20
        (for _array_element (LocalVariables|Getopenlist)
          (for _array_element_2 (Variables|/Game/Blueprint/Tiles/O_Tile.O_Tile_C|GetNeighbours _array_element)
            (Utilities|IsValid _array_element_2
              (:Is%20Valid
                (Utilities|Array|AddUnique (LocalVariables|GetSavedList) _array_element_2)))))
        (LocalVariables|Setopenlist (LocalVariables|GetSavedList)))))
  (return (LocalVariables|GetSavedList)))