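; Building component that spreads pollution onto nearby map tiles, with strength and range set by the building's state (Green, Dirty, Abbadoned).
; SwitchPollution first removes the old pollution, then selects the new values and applies them through UpdatePollution.
; Affected tiles are gathered uniquely within range of every tile the building occupies.
; Getters expose current strength and range; RemovePollution only loops over Dirty-range tiles without changing them.
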(fn SwitchPollution
  (params (BuildingState :type EBuildingState%20Enum :default "NewEnumerator0"))
  (Utilities|FlowControl|Sequence
    (:then_0
      ;[1 1 1] RemoveOldPollution
      (bind _asbp_game_instance (Utilities|Casting|CastToBP_GameInstance (Game|GetGameInstance)))
      (bind _asbp_base_building (Utilities|Casting|CastToBP_BaseBuilding (Components|GetOwner)))
      (bind _tiles (Default|FindTileswithBuilding (Variables|/Game/GameMode/BP_GameInstance.BP_GameInstance_C|GetMap _asbp_game_instance) _asbp_base_building))
      (for _array_element _tiles
        (bind _tiles_2 (CallFunction|GetTilesinRange _array_element (Variables|Default|GetCurrentRange)))
        (for _array_element_2 _tiles_2
          (Utilities|Array|AddUnique (LocalVariables|GetAffectedTiles) _array_element_2)))
      (Utilities|NegateInt (Variables|Default|GetCurrentPollution)
        (:%20%20
          (for _array_element_3 (LocalVariables|GetAffectedTiles)
            (Default|UpdatePollution _array_element_3 (Variables|Default|GetCurrentPollution))))))
    (:then_1
      ;[1 1 1] Clear List and Set new Values
      (Variables|Default|SetCurrentPollution (Utilities|Select :Index BuildingState :NewEnumerator0 (Variables|Pollution|GetStrengthClean) :NewEnumerator1 (Variables|Pollution|GetStrengthDirty) :NewEnumerator2 (Variables|Pollution|GetStrengthAbbadoned)))
      (Variables|Default|SetCurrentRange (Utilities|Select :Index BuildingState :NewEnumerator0 (Variables|Pollution|GetRangeClean) :NewEnumerator1 (Variables|Pollution|GetRangeDirty) :NewEnumerator2 (Variables|Pollution|GetRangeAbbadoned)))
      (Utilities|Array|Clear (LocalVariables|GetAffectedTiles))
      ;[1 1 1] AddNewPollution
      (bind _asbp_game_instance_2 (Utilities|Casting|CastToBP_GameInstance (Game|GetGameInstance)))
      (bind _asbp_base_building_2 (Utilities|Casting|CastToBP_BaseBuilding (Components|GetOwner)))
      (bind _tiles_3 (Default|FindTileswithBuilding (Variables|/Game/GameMode/BP_GameInstance.BP_GameInstance_C|GetMap _asbp_game_instance_2) _asbp_base_building_2))
      (for _array_element_4 _tiles_3
        (bind _tiles_4 (CallFunction|GetTilesinRange _array_element_4 (Variables|Default|GetCurrentRange)))
        (for _array_element_5 _tiles_4
          (Utilities|Array|AddUnique (LocalVariables|GetAffectedTiles) _array_element_5)))
      (for _array_element_6 (LocalVariables|GetAffectedTiles)
        (Default|UpdatePollution _array_element_6 (Variables|Default|GetCurrentPollution))))))

(fn RemovePollution
  (bind _asbp_game_instance (Utilities|Casting|CastToBP_GameInstance (Game|GetGameInstance)))
  (bind _tiles (CallFunction|GetTilesinRange (Default|GetTilefromWorldPosition (Variables|/Game/GameMode/BP_GameInstance.BP_GameInstance_C|GetMap _asbp_game_instance) (Transformation|GetActorLocation (Components|GetOwner))) (Variables|Pollution|GetRangeDirty)))
  (for _array_element _tiles
    _))

(fn GetCurrentPollution
  (return (Variables|Default|GetCurrentPollution)))

(fn GetPollutionRange
  (return (Variables|Default|GetCurrentRange)))