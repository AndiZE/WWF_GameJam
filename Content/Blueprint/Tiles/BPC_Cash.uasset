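; BPC_Cash is a tile component that supplies building income and handles the building's timed upgrade.
; GetIncome picks the clean, dirty or abandoned income from the given state, and GetUpgradeCost exposes the upgrade price.
; UpgradeBuilding starts a duration timer only when no upgrade is active.
; UpgradeFinished fires the finished dispatcher but sets the active flag to true again, so it never clears it.
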(fn GetIncome
  (params (State :type EBuildingState%20Enum :default "NewEnumerator0"))
  (return (Utilities|Select :Index State :NewEnumerator0 (Variables|Cash|GetIncomeClean) :NewEnumerator1 (Variables|Cash|GetIncomeDirty) :NewEnumerator2 (Variables|Cash|GetIncomeAbbadoned))))

(fn IsUpgrading
  (return (Variables|Default|GetupgradeActive)))

(fn UpgradeBuilding
  (if (not (Variables|Default|GetupgradeActive))
    (Variables|Default|SetupgradeActive true)
    (Utilities|Time|SetTimerbyEvent (EventDispatchers|CreateEvent :!event UpgradeFinished) (Variables|Cash|GetUpgradeDuration))))

(fn UpgradeFinished
  (Variables|Default|SetupgradeActive true)
  (Default|CallOnUpgradeFinished))

(fn GetUpgradeCost
  (return (Variables|Cash|GetUpgradeCost)))